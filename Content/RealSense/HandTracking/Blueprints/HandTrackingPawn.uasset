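; Pawn that visualizes Intel RealSense hand tracking for debugging.
; It starts the HandTracking camera on BeginPlay, then each Tick draws debug spheres at every joint of both hands.
; GetDebugPosition offsets tracked points ahead of and above the pawn and rotates them by control rotation.
; A Sphere component follows the right hand's mass center through the same transform, as a relative location.
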(event EventBeginPlay
  (Class|RealSenseComponent|StartCamera (Variables|Default|GetHandTracking)))

(event EventEndPlay
  (params (EndPlayReason :type EEndPlayReason%20Enum :default "Destroyed")))

(event EventTick
  (params (DeltaSeconds :type Float%20%28single-precision%29))
  (bind _handtracking (Variables|Default|GetHandTracking))
  (CallFunction|DrawDebugHand (Variables|/Script/RealSensePlugin.HandTrackingComponent|GetRealSenseHandLeft _handtracking))
  (CallFunction|DrawDebugHand (Variables|/Script/RealSensePlugin.HandTrackingComponent|GetRealSenseHandRight _handtracking))
  (bind _debuglocation (CallFunction|GetDebugPosition (.handmasscenterworld (Variables|/Script/RealSensePlugin.HandTrackingComponent|GetRealSenseHandRight _handtracking)) "0, 0, 0"))
  (Transformation|SetRelativeLocation (Variables|Default|GetSphere) _debuglocation false false))

(fn ConstructionScript)

(fn DrawDebugSphereActor
  (params (Location :type Vector) (Radius :type Float%20%28single-precision%29))
  (bind _debuglocation (CallFunction|GetDebugPosition Location (Transformation|GetActorLocation)))
  (Rendering|Debug|DrawDebugSphere _debuglocation Radius 12 "(R=0.000000,G=0.000000,B=0.000000,A=1.000000)" 0.0))

(fn DrawDebugHand
  (params (RealSenseHand :type Real%20Sense%20Hand%20Structure))
  (bind (_bisleft _bisright _id _bistracking _handmasscenterworld _palmorientation _palmradiusworld _openness _bishastrackedjoints _firedalertdata _jointwirst _jointcenter _jointthumbbase _jointthumbjt1 _jointthumbjt2 _jointthumbtip _jointindexbase _jointindexjt1 _jointindexjt2 _jointindextip _jointmiddlebase _jointmiddlejt1 _jointmiddlejt2 _jointmiddletip _jointringbase _jointringjt1 _jointringjt2 _jointringtip _jointpinkybase _jointpinkyjt1 _jointpinkyjt2 _jointpinkytip) (Utilities|Struct|BreakRealSenseHand RealSenseHand))
  (CallFunction|DrawDebugSphereActor (.PositionWorld (Utilities|Struct|BreakRealSenseJoint _jointwirst)) 4.0)
  (CallFunction|DrawDebugSphereActor (.PositionWorld (Utilities|Struct|BreakRealSenseJoint _jointcenter)) 2.0)
  (CallFunction|DrawDebugSphereActor (.PositionWorld (Utilities|Struct|BreakRealSenseJoint _jointthumbbase)) 1.0)
  (CallFunction|DrawDebugSphereActor (.PositionWorld (Utilities|Struct|BreakRealSenseJoint _jointthumbjt1)) 1.0)
  (CallFunction|DrawDebugSphereActor (.PositionWorld (Utilities|Struct|BreakRealSenseJoint _jointthumbjt2)) 1.0)
  (CallFunction|DrawDebugSphereActor (.PositionWorld (Utilities|Struct|BreakRealSenseJoint _jointthumbtip)) 1.0)
  (CallFunction|DrawDebugSphereActor (.PositionWorld (Utilities|Struct|BreakRealSenseJoint _jointindexbase)) 1.0)
  (CallFunction|DrawDebugSphereActor (.PositionWorld (Utilities|Struct|BreakRealSenseJoint _jointindexjt1)) 1.0)
  (CallFunction|DrawDebugSphereActor (.PositionWorld (Utilities|Struct|BreakRealSenseJoint _jointindexjt2)) 1.0)
  (CallFunction|DrawDebugSphereActor (.PositionWorld (Utilities|Struct|BreakRealSenseJoint _jointindextip)) 1.0)
  (CallFunction|DrawDebugSphereActor (.PositionWorld (Utilities|Struct|BreakRealSenseJoint _jointmiddlebase)) 1.0)
  (CallFunction|DrawDebugSphereActor (.PositionWorld (Utilities|Struct|BreakRealSenseJoint _jointmiddlejt1)) 1.0)
  (CallFunction|DrawDebugSphereActor (.PositionWorld (Utilities|Struct|BreakRealSenseJoint _jointmiddlejt2)) 1.0)
  (CallFunction|DrawDebugSphereActor (.PositionWorld (Utilities|Struct|BreakRealSenseJoint _jointmiddletip)) 1.0)
  (CallFunction|DrawDebugSphereActor (.PositionWorld (Utilities|Struct|BreakRealSenseJoint _jointringbase)) 1.0)
  (CallFunction|DrawDebugSphereActor (.PositionWorld (Utilities|Struct|BreakRealSenseJoint _jointringjt1)) 1.0)
  (CallFunction|DrawDebugSphereActor (.PositionWorld (Utilities|Struct|BreakRealSenseJoint _jointringjt2)) 1.0)
  (CallFunction|DrawDebugSphereActor (.PositionWorld (Utilities|Struct|BreakRealSenseJoint _jointringtip)) 1.0)
  (CallFunction|DrawDebugSphereActor (.PositionWorld (Utilities|Struct|BreakRealSenseJoint _jointpinkybase)) 1.0)
  (CallFunction|DrawDebugSphereActor (.PositionWorld (Utilities|Struct|BreakRealSenseJoint _jointpinkyjt1)) 1.0)
  (CallFunction|DrawDebugSphereActor (.PositionWorld (Utilities|Struct|BreakRealSenseJoint _jointpinkyjt2)) 1.0)
  (CallFunction|DrawDebugSphereActor (.PositionWorld (Utilities|Struct|BreakRealSenseJoint _jointpinkytip)) 1.0))

(fn GetDebugPosition
  (params (Location :type Vector) (ActorLocation :type Vector))
  (return (+ (Math|Vector|RotateVector (+ Location "150.000000,0.000000,50.000000") (Pawn|GetControlRotation :!class /Script/Engine.Pawn)) ActorLocation)))