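; HUD Blueprint in the RealSense HandTracking folder that shows live depth and color camera feeds on screen.
; It starts the CameraStream on BeginPlay.
; Each DrawHUD converts the stream's depth and color buffers into textures and draws them scaled down, with color offset horizontally from depth.
; It draws only the raw feeds, with no hand tracking data.
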(event Custom|DrawCameraDepthTexture
  (bind _camerastream (Variables|Default|GetCameraStream))
  ;[1 1 1] Add Camera Depth Texture
  (bind _returnvalue (Class|RealSenseBlueprintLibrary|DepthBuffertoTexture (Variables|/Script/RealSensePlugin.CameraStreamComponent|GetDepthBuffer _camerastream) (Variables|/Script/RealSensePlugin.CameraStreamComponent|GetDepthTexture _camerastream)))
  (Class|HUD|DrawTextureSimple _returnvalue 0.0 0.0 0.25 false))

(event Custom|DrawCameraRGBTexture
  (bind _camerastream (Variables|Default|GetCameraStream))
  ;[1 1 1] Add Camera RGB Texture
  (bind _returnvalue (Class|RealSenseBlueprintLibrary|ColorBuffertoTexture (Variables|/Script/RealSensePlugin.CameraStreamComponent|GetColorBuffer _camerastream) (Variables|/Script/RealSensePlugin.CameraStreamComponent|GetColorTexture _camerastream)))
  (Class|HUD|DrawTextureSimple _returnvalue 2e+02 0.0 0.25 false))

(event EventDrawHUD
  (params (SizeX :type Integer) (SizeY :type Integer))
  (CallFunction|DrawCameraDepthTexture)
  (CallFunction|DrawCameraRGBTexture))

(event EventBeginPlay
  (Class|RealSenseComponent|StartCamera (Variables|Default|GetCameraStream)))

(fn ConstructionScript)